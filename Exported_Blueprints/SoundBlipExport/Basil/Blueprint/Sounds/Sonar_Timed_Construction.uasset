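; Sonar_Timed_Construction is a trigger actor that plays a construction sound cue and animates a sonar decal around the first-person character's visits.
; Any overlap fades in the sound, then after a delay the character check sets InZone and starts a timeline lerping the decal between two transforms.
; Timeline updates schedule delayed replays while InZone holds, and fade the sound out once it clears.
; The Box hit event has no effect.
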(event OnComponentHit(Box)
  (params (HitComponent :type Primitive%20Component%20Object%20Reference) (OtherActor :type Actor%20Object%20Reference) (OtherComp :type Primitive%20Component%20Object%20Reference) (NormalImpulse :type Vector :default "0, 0, 0") (Hit :type Hit%20Result%20Structure%20%28by%20ref%29))
  (Utilities|FlowControl|Delay 2.0)
  (Utilities|Casting|CastToBoxComponent HitComponent))

(event Collision|EventActorEndOverlap
  (params (OtherActor :type Actor%20Object%20Reference))
  (Utilities|Casting|CastToFirstPersonCharacter OtherActor)
  (Variables|Default|SetinZone false))

(event Collision|EventActorBeginOverlap
  (params (OtherActor :type Actor%20Object%20Reference))
  (Audio|Components|Audio|FadeIn (Variables|Default|GetConstructionQue) 3.0 1.0 0.0 "Linear" :!class /Script/Engine.AudioComponent)
  (Utilities|FlowControl|Delay 2.0)
  (Utilities|Casting|CastToFirstPersonCharacter OtherActor)
  (Variables|Default|SetinZone true)
  (bind _newtrack_0 (Timeline|Timeline_0 PlayFromStart)
    (:Update
      (Transformation|SetRelativeTransform (Variables|Default|GetDecal) (Math|Transform|Lerp(Transform) (Variables|Default|GetNewVar_0) (Variables|Default|GetNewVar_1) _newtrack_0) false false)
      (if (Variables|Default|GetinZone)
        (Utilities|FlowControl|Delay 3.0)
        (Timeline|Timeline_0 PlayFromStart)
        (else
          (Audio|Components|Audio|FadeOut (Variables|Default|GetConstructionQue) 3.0 0.0 "Linear" :!class /Script/Engine.AudioComponent))))))

(fn ConstructionScript)